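; Prototype player card manager Blueprint, meant to build the player's card list from a deck of data assets.
; ConstructTheCards passes each DataAssetDeck entry to CreateCard and appends the result to GeneralCardList, then runs a counter loop that only increments Condition.
; CreateCard is a stub that returns without building a card.
; The events, construction script and NewFunction are empty, and nothing in this graph calls ConstructTheCards.
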(event EventBeginPlay)

(event Collision|EventActorBeginOverlap
  (params (OtherActor :type Actor%20Object%20Reference)))

(event EventTick
  (params (DeltaSeconds :type Float%20%28single-precision%29)))

(fn ConstructionScript)

(fn CreateCard
  (params (NewParam :type BPDA%20M02%20Card%20Object%20Reference))
  (return 0))

(fn NewFunction)

(fn ConstructtheCards
  (for _array_element (Variables|Default|GetDataAssetDeck)
    (bind _newparam1 (CallFunction|CreateCard _array_element))
    (Utilities|Array|Add (Variables|Default|GetGeneralCardList) _newparam1)
    (if (not (== (Variables|Default|GetCondition) 3)) :!label _label
      (Math|Integer|IncrementInt (Variables|Default|GetCondition)
        (:%20%20
          (goto _label))))))