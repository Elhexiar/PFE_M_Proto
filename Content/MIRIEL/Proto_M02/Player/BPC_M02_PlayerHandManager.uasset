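; Player component for the M02 prototype that manages the hand of cards.
; BeginPlay indexes the character's card holder actors; C draws from the current deck up to hand size, spawning an in-hand card with its widget filled from card data.
; Each card attaches to the next holder, aligned to the anchor's rotation.
; B test-swaps the first two holders' cards via ImmediateSwap; older curve-based arc layout code is left unused.
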(event EventBeginPlay
  (Utilities|FlowControl|Sequence
    (:then_0
      (bind _asbp_m02_rtscontroler (CallFunction|GetM02PlayerController))
      (Variables|Default|SetPlayerController _asbp_m02_rtscontroler)
      (bind _bp_m02_rtsplayer_character_2 (CallFunction|GetM02PlayerCharacter))
      (Variables|Default|SetPlayerCharacter _bp_m02_rtsplayer_character_2)
      (Variables|Default|SetCurrent%20Player%20Deck%20Reference (Variables|/Game/MIRIEL/Proto_M02/Player/BPC_M02_CardManager.BPC_M02_CardManager_C|GetCurrentPlayerDeck (Variables|/Game/MIRIEL/Proto_M02/Player/BP_M02_RTSControler.BP_M02_RTSControler_C|GetPlayerCardManager (Variables|Default|GetPlayerController))))
      (for _array_element (Components|GetChildrenComponents (Variables|/Game/MIRIEL/Proto_M02/Player/BP_M02_RTSPlayerCharacter2.BP_M02_RTSPlayerCharacter2_C|GetCardHolder_01 (Variables|Default|GetPlayerCharacter)) true)
        (bind _aschild_actor_component (Utilities|Casting|CastToChildActorComponent _array_element))
        (bind _asbp_m02_card_holder (Utilities|Casting|CastToBP_M02_CardHolder (Variables|/Script/Engine.ChildActorComponent|GetChildActor _aschild_actor_component)))
        (Utilities|Map|Add (Variables|Default|GetCardHolderList) (Variables|/Game/MIRIEL/Proto_M02/Cards/InHand/BP_M02_CardHolder.BP_M02_CardHolder_C|GetIndex _asbp_m02_card_holder) _asbp_m02_card_holder)))))

(event EventTick
  (params (DeltaSeconds :type Float%20%28single-precision%29)))

(event Input|KeyboardEvents|C
  (params (Key :type Key%20Structure :default "None"))
  (:Pressed
    (Utilities|FlowControl|Sequence
      (:then_0
        (if (> (Variables|Default|GetHandSize) (Utilities|Array|Length (Variables|Default|GetInHandCardActorList)))
          (bind (_pickedcard _isnotempty) (Default|PickTopCard (Variables|Default|GetCurrent%20Player%20Deck%20Reference)))
          (if _isnotempty
            (Utilities|Array|Insert (Variables|Default|GetPlayerCardList) _pickedcard)
            (CallFunction|BuildinHandCardActor (Variables|/Script/PFE_M_Proto.Card|GetInHandActorClass _pickedcard) _pickedcard)))))))

(event Input|KeyboardEvents|B
  (params (Key :type Key%20Structure :default "None"))
  (:Pressed
    (CallFunction|ImmediateSwap (.Value (Utilities|Map|Find (Variables|Default|GetCardHolderList) 0)) (.Value (Utilities|Map|Find (Variables|Default|GetCardHolderList) 1)))))

(fn BuildinHandCardActor
  (params (Class :type Actor%20Class%20Reference) (Card%20Actor :type Card%20Object%20Reference))
  (bind _playercharacter (Variables|Default|GetPlayerCharacter))
  (bind _card_anchor (Variables|/Game/MIRIEL/Proto_M02/Player/BP_M02_RTSPlayerCharacter2.BP_M02_RTSPlayerCharacter2_C|GetCard%20Anchor _playercharacter))
  (bind _returnvalue (Transformation|GetWorldTransform _card_anchor))
  (Utilities|FlowControl|Sequence
    (:then_0
      (bind _asbp_m02_summon_card (Utilities|Casting|CastToBP_M02_SummonCard Card%20Actor))
      (LocalVariables|Setcard%20object _asbp_m02_summon_card)
      (bind _returnvalue_2 (Game|SpawnActorfromClass Class _returnvalue "Undefined" "MultiplyWithRoot" 0 0))
      (bind _asbp_m02_in_hand_card (Utilities|Casting|CastToBP_M02_InHandCard _returnvalue_2))
      (bind _output_get (LocalVariables|SetCardActor _asbp_m02_in_hand_card))
      (Utilities|Array|Insert (Variables|Default|GetInHandCardActorList) _output_get)
      (Transformation|AttachComponentToComponent _output_get _card_anchor "None" "KeepRelative" "KeepRelative" "KeepRelative" false)
      (Transformation|SetActorTransform _output_get _returnvalue))
    (:then_1
      (bind _aswbp_in_hand_card_widget (Utilities|Casting|CastToWBP_InHandCardWidget (UserInterface|GetWidget (Variables|/Game/MIRIEL/Proto_M02/Cards/InHand/BP_M02_InHandCard.BP_M02_InHandCard_C|GetCardWidget (LocalVariables|GetCardActor)))))
      (LocalVariables|SetCardActorWidget _aswbp_in_hand_card_widget))
    (:then_2
      (Appearance|SetColorandOpacity (Variables|/Game/MIRIEL/Proto_M02/Cards/InHand/WBP_InHandCardWidget.WBP_InHandCardWidget_C|GetBackgroundImage (LocalVariables|GetCardActorWidget)) (Math|Conversions|ToLinearColor(Color) (Variables|/Game/MIRIEL/Proto_M02/Cards/BP_M02_SummonCard.BP_M02_SummonCard_C|GetTestColor (LocalVariables|Getcard%20object))) :!class /Script/UMG.Image)
      (Variables|/Script/UMG.TextBlock|SetText (Variables|/Game/MIRIEL/Proto_M02/Cards/InHand/WBP_InHandCardWidget.WBP_InHandCardWidget_C|GetMainText (LocalVariables|GetCardActorWidget)) (Utilities|Text|ToText(String) (Variables|/Script/PFE_M_Proto.Card|GetName (LocalVariables|Getcard%20object)))))
    (:then_3
      (Variables|/Game/MIRIEL/Proto_M02/Cards/InHand/BP_M02_CardHolder.BP_M02_CardHolder_C|SetInHandCardRef (.Value (Utilities|Map|Find (Variables|Default|GetCardHolderList) (- (Utilities|Array|Length (Variables|Default|GetInHandCardActorList)) 1))) (LocalVariables|GetCardActor))
      (bind _values (Utilities|Map|Values (Variables|Default|GetCardHolderList)))
      (for _array_element _values
        (if (Utilities|IsValid (Variables|/Game/MIRIEL/Proto_M02/Cards/InHand/BP_M02_CardHolder.BP_M02_CardHolder_C|GetInHandCardRef _array_element))
          (Variables|/Game/MIRIEL/Proto_M02/Cards/InHand/BP_M02_InHandCard.BP_M02_InHandCard_C|SetHolder (Variables|/Game/MIRIEL/Proto_M02/Cards/InHand/BP_M02_CardHolder.BP_M02_CardHolder_C|GetInHandCardRef _array_element) _array_element)
          (Transformation|DetachFromActor (Variables|/Game/MIRIEL/Proto_M02/Cards/InHand/BP_M02_CardHolder.BP_M02_CardHolder_C|GetInHandCardRef _array_element) "KeepRelative" "KeepRelative" "KeepRelative")
          (Transformation|AttachActorToActor (Variables|/Game/MIRIEL/Proto_M02/Cards/InHand/BP_M02_CardHolder.BP_M02_CardHolder_C|GetInHandCardRef _array_element) _array_element "None" "KeepRelative" "KeepRelative" "KeepRelative" true)
          (Transformation|SetActorLocation (Variables|/Game/MIRIEL/Proto_M02/Cards/InHand/BP_M02_CardHolder.BP_M02_CardHolder_C|GetInHandCardRef _array_element) (Transformation|GetActorLocation _array_element) false false)
          (CallFunction|ResetRotation (Variables|/Game/MIRIEL/Proto_M02/Cards/InHand/BP_M02_CardHolder.BP_M02_CardHolder_C|GetInHandCardRef _array_element)))))))

(fn ReorganiseHandV1
  (bind _returnvalue (/ 1.0 2.0))
  (bind _inhandcardactorlist (Variables|Default|GetInHandCardActorList))
  (for (_array_element _array_index) _inhandcardactorlist
    (if (== (Utilities|Array|Length _inhandcardactorlist) 1)
      (Transformation|SetActorTransform _array_element (Transformation|GetWorldTransform (Variables|/Game/MIRIEL/Proto_M02/Player/BP_M02_RTSPlayerCharacter2.BP_M02_RTSPlayerCharacter2_C|GetCard%20Anchor (Variables|Default|GetPlayerCharacter))))
      (Transformation|AddActorLocalOffset _array_element (Math|Vector|MakeVector (Math|Float|Lerp (* (Variables|Default|GetDepthHandLength) -1.0) (Variables|Default|GetDepthHandLength) _returnvalue) (Math|Float|Lerp (* (Variables|Default|GetHorizontalHandLength) -1.0) (Variables|Default|GetHorizontalHandLength) _returnvalue) (Math|Float|Lerp 0.0 (Variables|Default|GetArcOffset) (Math|Curves|GetFloatValue (Variables|Default|GetHandCurve) _returnvalue))) false false)
      (else
        (Transformation|SetActorTransform _array_element (Transformation|GetWorldTransform (Variables|/Game/MIRIEL/Proto_M02/Player/BP_M02_RTSPlayerCharacter2.BP_M02_RTSPlayerCharacter2_C|GetCard%20Anchor (Variables|Default|GetPlayerCharacter))))
        (Transformation|AddActorLocalOffset _array_element (Math|Vector|MakeVector (Math|Float|Lerp (* (Variables|Default|GetDepthHandLength) -1.0) (Variables|Default|GetDepthHandLength) (/ (Math|Conversions|ToFloat(Integer) _array_index) (- (Math|Conversions|ToFloat(Integer) (Utilities|Array|Length (Variables|Default|GetInHandCardActorList))) 1.0))) (Math|Float|Lerp (* (Variables|Default|GetHorizontalHandLength) -1.0) (Variables|Default|GetHorizontalHandLength) (/ (Math|Conversions|ToFloat(Integer) _array_index) (- (Math|Conversions|ToFloat(Integer) (Utilities|Array|Length (Variables|Default|GetInHandCardActorList))) 1.0))) (Math|Float|Lerp 0.0 (Variables|Default|GetArcOffset) (Math|Curves|GetFloatValue (Variables|Default|GetHandCurve) (/ (Math|Conversions|ToFloat(Integer) _array_index) (- (Math|Conversions|ToFloat(Integer) (Utilities|Array|Length (Variables|Default|GetInHandCardActorList))) 1.0))))) false false)))))

(fn ReorganiseHandV2)

(fn ImmediateSwap
  (params (CardHolderA :type BP%20M02%20Card%20Holder%20Object%20Reference) (CardHolderB :type BP%20M02%20Card%20Holder%20Object%20Reference))
  (if (Utilities|IsValid (Variables|/Game/MIRIEL/Proto_M02/Cards/InHand/BP_M02_CardHolder.BP_M02_CardHolder_C|GetInHandCardRef CardHolderA))
    (LocalVariables|SetActor%20A (Variables|/Game/MIRIEL/Proto_M02/Cards/InHand/BP_M02_CardHolder.BP_M02_CardHolder_C|GetInHandCardRef CardHolderA))
    (else
      (Development|PrintString "A is not valid")))
  (if (Utilities|IsValid (Variables|/Game/MIRIEL/Proto_M02/Cards/InHand/BP_M02_CardHolder.BP_M02_CardHolder_C|GetInHandCardRef CardHolderB))
    (LocalVariables|SetActor%20B (Variables|/Game/MIRIEL/Proto_M02/Cards/InHand/BP_M02_CardHolder.BP_M02_CardHolder_C|GetInHandCardRef CardHolderB))
    (else
      (Development|PrintString "b is not valid")))
  (Utilities|FlowControl|Sequence
    (:then_0
      (if (Utilities|IsValid (LocalVariables|GetActor%20A))
        (Transformation|DetachFromActor (LocalVariables|GetActor%20A) "KeepWorld" "KeepWorld" "KeepWorld")
        (Variables|/Game/MIRIEL/Proto_M02/Cards/InHand/BP_M02_CardHolder.BP_M02_CardHolder_C|SetInHandCardRef CardHolderA 0)
        (Transformation|AttachActorToActor (LocalVariables|GetActor%20A) CardHolderB "None" "KeepRelative" "KeepRelative" "KeepRelative" false)
        (Variables|/Game/MIRIEL/Proto_M02/Cards/InHand/BP_M02_CardHolder.BP_M02_CardHolder_C|SetInHandCardRef CardHolderB (LocalVariables|GetActor%20A))
        (Variables|/Game/MIRIEL/Proto_M02/Cards/InHand/BP_M02_InHandCard.BP_M02_InHandCard_C|SetHolder (LocalVariables|GetActor%20A) CardHolderB)
        (Transformation|SetActorLocation (Variables|/Game/MIRIEL/Proto_M02/Cards/InHand/BP_M02_CardHolder.BP_M02_CardHolder_C|GetInHandCardRef CardHolderB) (Transformation|GetActorLocation CardHolderB) false false)
        (CallFunction|ResetRotation (Variables|/Game/MIRIEL/Proto_M02/Cards/InHand/BP_M02_CardHolder.BP_M02_CardHolder_C|GetInHandCardRef CardHolderB))
        (Development|PrintString (Utilities|String|Append "Actor " (Utilities|GetDisplayName (Variables|/Game/MIRIEL/Proto_M02/Cards/InHand/BP_M02_CardHolder.BP_M02_CardHolder_C|GetInHandCardRef CardHolderB)) "is now in holder " (Utilities|GetDisplayName CardHolderB)))
        (else
          (if (Utilities|IsValid (LocalVariables|GetActor%20B)) :!label _label
            (Transformation|DetachFromActor (LocalVariables|GetActor%20B) "KeepWorld" "KeepWorld" "KeepWorld")
            (Transformation|AttachActorToActor (LocalVariables|GetActor%20B) CardHolderA "None" "KeepRelative" "KeepRelative" "KeepRelative" false)
            (Variables|/Game/MIRIEL/Proto_M02/Cards/InHand/BP_M02_CardHolder.BP_M02_CardHolder_C|SetInHandCardRef CardHolderA (LocalVariables|GetActor%20B))
            (Variables|/Game/MIRIEL/Proto_M02/Cards/InHand/BP_M02_InHandCard.BP_M02_InHandCard_C|SetHolder (LocalVariables|GetActor%20B) CardHolderA)
            (Transformation|SetActorLocation (Variables|/Game/MIRIEL/Proto_M02/Cards/InHand/BP_M02_CardHolder.BP_M02_CardHolder_C|GetInHandCardRef CardHolderA) (Transformation|GetActorLocation CardHolderA) false false)
            (CallFunction|ResetRotation (Variables|/Game/MIRIEL/Proto_M02/Cards/InHand/BP_M02_CardHolder.BP_M02_CardHolder_C|GetInHandCardRef CardHolderA))
            (Development|PrintString (Utilities|String|Append "Actor " (Utilities|GetDisplayName (Variables|/Game/MIRIEL/Proto_M02/Cards/InHand/BP_M02_CardHolder.BP_M02_CardHolder_C|GetInHandCardRef CardHolderA)) "is now in holder " (Utilities|GetDisplayName CardHolderA)))))))
    (:then_1
      (Development|PrintString (Utilities|String|Append " trying to put Actor " (Utilities|GetDisplayName (LocalVariables|GetActor%20B)) " in holder " (Utilities|GetDisplayName CardHolderA)))
      (goto _label))))

(fn ResetRotation
  (params (Card%20Actor :type BP%20M02%20in%20Hand%20Card%20Object%20Reference))
  (Transformation|SetActorRotation Card%20Actor (.rotation (Transformation|GetWorldTransform (Variables|/Game/MIRIEL/Proto_M02/Player/BP_M02_RTSPlayerCharacter2.BP_M02_RTSPlayerCharacter2_C|GetCard%20Anchor (Variables|Default|GetPlayerCharacter))))))