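; Player component for the M02 card prototype that builds the overall card pool and the player's current deck on BeginPlay.
; Card data assets become runtime objects in the overall deck, with summon cards copying their asset's fields.
; The current deck draws ten random entries from that pool with replacement, sharing the same card objects and inserting each at a random index.
; Active card building and building from a card list are unfinished stubs.
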(event EventTick
  (params (DeltaSeconds :type Float%20%28single-precision%29)))

(event EventBeginPlay
  (Utilities|FlowControl|Sequence
    (:then_0
      (bind _deck (CallFunction|BuildDeckfromDAList (Variables|Default|GetgeneralDA_CardList)))
      (Variables|Default|SetOverallDeck _deck))
    (:then_1
      (bind _built_deck (CallFunction|BuildDeckwithNRandomCards 10))
      (Variables|Default|SetCurrentPlayerDeck _built_deck))))

(fn BuildDeckfromDAList
  (params (dataAssetList :type Array%20of%20BPDA%20M02%20Card%20Object%20References))
  (bind _returnvalue (Game|ConstructObjectfromClass "/Game/MIRIEL/Proto_M02/Cards/BP_M02_Deck.BP_M02_Deck_C"))
  (for _array_element dataAssetList
    (bind _asbpda_m02_summon_card (Utilities|Casting|CastToBPDA_M02_SummonCard _array_element)
      (:then
        (bind _summoncard (CallFunction|BuildSummonCardfromDA _asbpda_m02_summon_card))
        (Default|AddTopCard _returnvalue _summoncard))
      (:CastFailed
        (bind _asbpda_m02_active_card (Utilities|Casting|CastToBPDA_M02_ActiveCard _array_element))
        (bind _activecard (CallFunction|BuildActiveCardfromDA _asbpda_m02_active_card))
        (Default|AddTopCard _returnvalue _activecard))))
  (return _returnvalue))

(fn BuildSummonCardfromDA
  (params (dataAsset :type BPDA%20M02%20Summon%20Card%20Object%20Reference))
  (LocalVariables|SetDataAssetToBuildFrom dataAsset)
  (bind _returnvalue (Game|ConstructObjectfromClass "/Game/MIRIEL/Proto_M02/Cards/BP_M02_SummonCard.BP_M02_SummonCard_C"))
  (Variables|/Script/PFE_M_Proto.Card|SetName _returnvalue (Variables|/Game/MIRIEL/Proto_M02/Cards/BPDA/BPDA_M02_Card.BPDA_M02_Card_C|GetName (LocalVariables|GetDataAssetToBuildFrom)))
  (Variables|/Script/PFE_M_Proto.Card|SetCost _returnvalue (Variables|/Game/MIRIEL/Proto_M02/Cards/BPDA/BPDA_M02_Card.BPDA_M02_Card_C|GetCost (LocalVariables|GetDataAssetToBuildFrom)))
  (Variables|/Script/PFE_M_Proto.Card|SetDescription _returnvalue (Variables|/Game/MIRIEL/Proto_M02/Cards/BPDA/BPDA_M02_Card.BPDA_M02_Card_C|GetDescription (LocalVariables|GetDataAssetToBuildFrom)))
  (Variables|/Script/PFE_M_Proto.Card|SetInHandActorClass _returnvalue (Variables|/Game/MIRIEL/Proto_M02/Cards/BPDA/BPDA_M02_Card.BPDA_M02_Card_C|GetInHandModel (LocalVariables|GetDataAssetToBuildFrom)))
  (Variables|/Game/MIRIEL/Proto_M02/Cards/BP_M02_SummonCard.BP_M02_SummonCard_C|SetTestColor _returnvalue (Variables|/Game/MIRIEL/Proto_M02/Cards/BPDA/BPDA_M02_SummonCard.BPDA_M02_SummonCard_C|GetTestColor (LocalVariables|GetDataAssetToBuildFrom)))
  (return _returnvalue))

(fn BuildActiveCardfromDA
  (params (dataAsset :type BPDA%20M02%20Active%20Card%20Object%20Reference))
  (LocalVariables|SetDataAssetToBuildFrom dataAsset)
  (Game|ConstructObjectfromClass "/Game/MIRIEL/Proto_M02/Cards/BP_M02_ActiveCard.BP_M02_ActiveCard_C")
  (Development|PrintString "Build Active Card from DA not implemented yet")
  (return 0))

(fn BuildDeckwithNRandomCards
  (params (n%20size :type Integer))
  (bind _overalldeck (Variables|Default|GetOverallDeck))
  (bind _cardlist (Variables|/Game/MIRIEL/Proto_M02/Cards/BP_M02_Deck.BP_M02_Deck_C|GetcardList _overalldeck))
  (bind _returnvalue (Game|ConstructObjectfromClass "/Game/MIRIEL/Proto_M02/Cards/BP_M02_Deck.BP_M02_Deck_C"))
  (for _index (range 1 n%20size)
    (Default|AddCardatRandomIndex _returnvalue (Utilities|Array|Get(acopy) _cardlist (.OutIndex (Utilities|Array|Random _cardlist)))))
  (return _returnvalue))

(fn BuildDeckfromCardList
  (Development|PrintString "Build Deck from Card List not implemented yet"))