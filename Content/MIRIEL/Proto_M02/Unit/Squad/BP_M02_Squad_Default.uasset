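; Default squad actor for the M02 prototype that spawns and commands a square formation of units.
; The construction script fills a grid-to-class map from the unit catalogue, overriding two partial rows and four cells with other unit types.
; BeginPlay spawns each valid cell's unit, centred on the root, plus a handler attached to the squad and linked to that unit.
; MoveAllUnits tells every handler to move its unit.
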(event Custom|Move%20All%20Units
  (for _array_element (Variables|Default|GetHandlerList)
    (Default|MoveUnit _array_element)))

(event EventBeginPlay
  (bind _self self)
  (bind _spacinglength (Variables|Default|GetSpacingLength))
  (bind _formationlength (Variables|Default|GetFormationLength))
  (bind _returnvalue (Math|Conversions|ToFloat(Integer) _formationlength))
  (bind _defaultsceneroot (Variables|Default|GetDefaultSceneRoot _self))
  (bind _returnvalue_2 (Transformation|GetWorldLocation _defaultsceneroot))
  (|CallParentFunction)
  (for _index (range 0 (- (Variables|Default|GetFormationLength) -1))
    (for _index_2 (range 0 (- (Variables|Default|GetFormationLength) -1))
      (if (Utilities|IsValidClass (.Value (Utilities|Map|Find (Variables|Default|GetSquadLayout) (Math|Vector2D|MakeVector2D (Math|Conversions|ToFloat(Integer) _index_2) (Math|Conversions|ToFloat(Integer) _index)))))
        (Development|PrintString (Utilities|String|Append "Spawn actor [" (Utilities|String|ToString(Integer) _index_2) "][" (Utilities|String|ToString(Integer) _index) "] with formation length " (Utilities|String|ToString(Float) 0.0)))
        (bind _returnvalue_3 (Game|SpawnActorfromClass (.Value (Utilities|Map|Find (Variables|Default|GetSquadLayout) (Math|Vector2D|MakeVector2D (Math|Conversions|ToFloat(Integer) _index_2) (Math|Conversions|ToFloat(Integer) _index)))) (Math|Transform|MakeTransform (Math|Vector|MakeVector (|((xOrigin-(((fLength-1)*fUnit)/2))+(index*fUnit)) _returnvalue _spacinglength (Math|Conversions|ToFloat(Integer) _index) (.x _returnvalue_2)) (|((yOrigin+(((fLength-1)*fUnit)/2))-(index*fUnit)) _returnvalue _spacinglength (Math|Conversions|ToFloat(Integer) _index_2) (.y _returnvalue_2)) 5e+02) "0, 0, 0" "1.000000,1.000000,1.000000") "Undefined" "MultiplyWithRoot" 0 0))
        (Utilities|Array|Add (Variables|Default|GetUnitList) _returnvalue_3)
        (bind _returnvalue_4 (Game|SpawnActorfromClass "/Game/MIRIEL/Proto_M02/Unit/Squad/SquadSingleUnitHandler.SquadSingleUnitHandler_C" (Math|Transform|MakeTransform (Math|Vector|MakeVector (|((xOrigin-(((fLength-1)*fUnit)/2))+(index*fUnit)) _returnvalue _spacinglength (Math|Conversions|ToFloat(Integer) _index) (.x _returnvalue_2)) (|((yOrigin+(((fLength-1)*fUnit)/2))-(index*fUnit)) _returnvalue _spacinglength (Math|Conversions|ToFloat(Integer) _index_2) (.y _returnvalue_2)) 5e+02) "0, 0, 0" "1.000000,1.000000,1.000000") "Undefined" "MultiplyWithRoot" 0 0))
        (Utilities|Array|Add (Variables|Default|GetHandlerList) _returnvalue_4)
        (Transformation|AttachActorToActor _returnvalue_4 self "None" "KeepRelative" "KeepRelative" "KeepRelative" true)
        (Variables|/Game/MIRIEL/Proto_M02/Unit/Squad/SquadSingleUnitHandler.SquadSingleUnitHandler_C|SetUnitToHandle _returnvalue_4 _returnvalue_3)))))

(event Collision|EventActorBeginOverlap
  (params (OtherActor :type Actor%20Object%20Reference))
  (|CallParentFunction OtherActor) ; This node is disabled and will not be called.\nDrag off pins to build functionality.
)

(event EventTick
  (params (DeltaSeconds :type Float%20%28single-precision%29))
  (|CallParentFunction DeltaSeconds) ; This node is disabled and will not be called.\nDrag off pins to build functionality.
)

(fn ConstructionScript
  (|CallParentFunction)
  (for _index (range 0 (- (Variables|Default|GetFormationLength) 1))
    (for _index_2 (range 0 (- (Variables|Default|GetFormationLength) 1))
      (Utilities|Map|Add (Variables|Default|GetSquadLayout) (Math|Vector2D|MakeVector2D (Math|Conversions|ToFloat(Integer) _index_2) (Math|Conversions|ToFloat(Integer) _index)) (.Value (Utilities|Map|Find (Variables|Default|GetSquadUnitCatalogue) 0)))))
  (for _index_3 (range 31 32)
    (for _index_4 (range 15 47)
      (Utilities|Map|Add (Variables|Default|GetSquadLayout) (Math|Vector2D|MakeVector2D (Math|Conversions|ToFloat(Integer) _index_4) (Math|Conversions|ToFloat(Integer) _index_3)) (.Value (Utilities|Map|Find (Variables|Default|GetSquadUnitCatalogue) 1)))))
  (Utilities|Map|Add (Variables|Default|GetSquadLayout) (Math|Vector2D|MakeVector2D 15.0 3e+01) "/Game/MIRIEL/Proto_M02/Unit/Old/BP_M02_TestUnit_Red.BP_M02_TestUnit_Red_C")
  (Utilities|Map|Add (Variables|Default|GetSquadLayout) (Math|Vector2D|MakeVector2D 16.0 3e+01) "/Game/MIRIEL/Proto_M02/Unit/Old/BP_M02_TestUnit_Red.BP_M02_TestUnit_Red_C")
  (Utilities|Map|Add (Variables|Default|GetSquadLayout) (Math|Vector2D|MakeVector2D 46.0 3e+01) "/Game/MIRIEL/Proto_M02/Unit/Old/BP_M02_TestUnit_Red.BP_M02_TestUnit_Red_C")
  (Utilities|Map|Add (Variables|Default|GetSquadLayout) (Math|Vector2D|MakeVector2D 47.0 3e+01) "/Game/MIRIEL/Proto_M02/Unit/Old/BP_M02_TestUnit_Red.BP_M02_TestUnit_Red_C"))