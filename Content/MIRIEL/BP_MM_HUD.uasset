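; HUD Blueprint that provides RTS-style drag-box selection of BP_MyFirstUnit actors.
; While IsDrawing is set, DrawHUD draws a translucent green rectangle from InitMousePos to the current mouse position.
; Each such frame it hides old selection markers, stores the units inside the rectangle in BP_RTSControler's SelectedUnitList, and shows their markers.
; A separate DrawDragBox function draws line edges and prints debug text; the event graph never calls it.
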(event EventBeginPlay)

(event EventTick
  (params (DeltaSeconds :type Float%20%28single-precision%29)))

(event EventDrawHUD
  (params (SizeX :type Integer) (SizeY :type Integer))
  (bind _returnvalue (Game|GetPlayerController 0))
  (bind _returnvalue_2 (Game|GetPlayerController 0))
  (bind _initmousepos (Variables|Default|GetInitMousePos))
  (bind (_locationx _locationy) (Game|Player|GetMousePosition _returnvalue))
  (bind (_locationx_2 _locationy_2) (Game|Player|GetMousePosition _returnvalue_2))
  (if (Variables|Default|GetIsDrawing)
    (HUD|DrawRect "(R=0.231422,G=1.000000,B=0.267655,A=0.182000)" (.x _initmousepos) (.y _initmousepos) (- _locationx (.x _initmousepos)) (- _locationy (.y _initmousepos)))
    ;[1 1 1] Dirty unselect
    (bind _asbp_rtscontroler (Utilities|Casting|CastToBP_RTSControler (Game|GetPlayerController 0)))
    (for _array_element (Variables|/Game/MIRIEL/BP_RTSControler.BP_RTSControler_C|GetSelectedUnitList _asbp_rtscontroler)
      (Rendering|SetVisibility (Variables|/Game/MIRIEL/Unit/BP_MyFirstUnit.BP_MyFirstUnit_C|GetSelection%20Marker _array_element) false false))
    ;[1 1 1] Dirty select
    (bind _filteredarray (Utilities|Array|FilterArray (Class|HUD|GetActorsinSelectionRectangle "/Game/MIRIEL/Unit/BP_MyFirstUnit.BP_MyFirstUnit_C" (Math|Vector2D|MakeVector2D (.x _initmousepos) (.y _initmousepos)) (Math|Vector2D|MakeVector2D _locationx_2 _locationy_2) false false) "/Game/MIRIEL/Unit/BP_MyFirstUnit.BP_MyFirstUnit_C"))
    (bind _output_get (Variables|/Game/MIRIEL/BP_RTSControler.BP_RTSControler_C|SetSelectedUnitList _asbp_rtscontroler _filteredarray))
    (for _array_element_2 _output_get
      (Rendering|SetVisibility (Variables|/Game/MIRIEL/Unit/BP_MyFirstUnit.BP_MyFirstUnit_C|GetSelection%20Marker _array_element_2) true false))))

(fn ConstructionScript)

(fn DrawDragBox
  (params (Initial%20mouse%20Pos :type Vector%202D%20Structure))
  (bind _returnvalue (Game|GetPlayerController 0))
  (bind _context (Variables|Default|GetContext))
  (bind (_locationx _locationy) (Game|Player|GetMousePosition _returnvalue))
  (Class|WidgetBlueprintLibrary|DrawLine _context (Math|Vector2D|MakeVector2D (.x Initial%20mouse%20Pos) (.y Initial%20mouse%20Pos)) (Math|Vector2D|MakeVector2D _locationx (.y Initial%20mouse%20Pos)) (Variables|Default|GetTint) true (Variables|Default|GetThickness))
  (Class|WidgetBlueprintLibrary|DrawLine _context (Math|Vector2D|MakeVector2D _locationx (.y Initial%20mouse%20Pos)) (Math|Vector2D|MakeVector2D _locationx _locationy) (Variables|Default|GetTint))
  (Class|WidgetBlueprintLibrary|DrawLine _context (Math|Vector2D|MakeVector2D _locationx _locationy) (Math|Vector2D|MakeVector2D (.x Initial%20mouse%20Pos) _locationy) (Variables|Default|GetTint))
  (Class|WidgetBlueprintLibrary|DrawLine _context (Math|Vector2D|MakeVector2D (.x Initial%20mouse%20Pos) _locationy) (Math|Vector2D|MakeVector2D _locationx _locationy) (Variables|Default|GetTint))
  (Development|PrintString "draw to "))