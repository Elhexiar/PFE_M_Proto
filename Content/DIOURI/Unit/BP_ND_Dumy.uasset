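; BP_ND_Dumy is a selectable dummy enemy unit with a health bar widget and an on-screen enemy info box.
; Cursor hover on the cylinder swaps the mesh to a selection-marker material, and SetSelected keeps that highlight and shows or hides the info box.
; Tick feeds DumyHealth to both displays against a hardcoded maximum and sets the health bar's relative yaw from the player character's yaw.
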(event OnBeginCursorOver(Cylinder)
  (params (TouchedComponent :type Primitive%20Component%20Object%20Reference))
  (Rendering|Material|SetMaterial (Variables|Character|GetMesh) 0 "/Game/DIOURI/Material/M_ND_SelectionMarker.M_ND_SelectionMarker")
  (Variables|Default|SetHovering true))

(event OnEndCursorOver(Cylinder)
  (params (TouchedComponent :type Primitive%20Component%20Object%20Reference))
  (if (not (Variables|Default|GetSelected))
    (Rendering|Material|SetMaterial (Variables|Character|GetMesh) 0 "/Game/StarterContent/Materials/M_Metal_Copper.M_Metal_Copper")
    (Variables|Default|SetHovering false)))

(event Custom|SetSelected
  (params (selected :type Boolean))
  (bind _enemyboxui (Variables|Default|GetEnemyBoxUI))
  (if selected
    (Variables|Default|SetSelected true)
    (Rendering|Material|SetMaterial (Variables|Character|GetMesh) 0 "/Game/DIOURI/Material/M_ND_SelectionMarker.M_ND_SelectionMarker")
    (Widget|SetVisibility _enemyboxui "Visible")
    (else
      (Variables|Default|SetSelected false)
      (Rendering|Material|SetMaterial (Variables|Character|GetMesh) 0 "/Game/StarterContent/Materials/M_Metal_Copper.M_Metal_Copper")
      (Widget|SetVisibility _enemyboxui "Hidden"))))

(event EventBeginPlay
  (Variables|/Script/Engine.PlayerController|SetbEnableMouseOverEvents (Game|GetPlayerController 0) true)
  (bind _returnvalue (Game|ConstructObjectfromClass "/Game/DIOURI/UI/WBP_EnemyBox.WBP_EnemyBox_C"))
  (bind _output_get (Variables|Default|SetEnemyBoxUI _returnvalue))
  (UserInterface|Viewport|AddtoViewport _output_get 0)
  (Widget|SetVisibility _output_get "Hidden"))

(event EventTick
  (params (DeltaSeconds :type Float%20%28single-precision%29))
  (bind _aswb_enemy_health_bar (Utilities|Casting|CastToWB_EnemyHealthBar (UserInterface|GetWidget (Variables|Default|GetHealthBarWidget))))
  (Progress|SetPercent (Variables|/Game/DIOURI/UI/WB_EnemyHealthBar.WB_EnemyHealthBar_C|GetTestHealthBar _aswb_enemy_health_bar) (/ (Variables|Default|GetDumyHealth) 1e+04))
  (Default|ShowStats (Variables|Default|GetEnemyBoxUI) (/ (Variables|Default|GetDumyHealth) 1e+04) (Variables|Default|GetDumyHealth))
  (Transformation|SetRelativeRotation (Variables|Default|GetHealthBarWidget) (Math|Rotator|MakeRotator 0.0 0.0 (.yaw (Transformation|GetActorRotation (Game|GetPlayerCharacter 0)))) false false))

(fn ConstructionScript)